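; BP_PlayerController is a player controller that handles basic movement and mouse look for the player's pawn.
; MoveForward and MoveRight axis inputs add movement input to player pawn 0 along the controller's own forward and right vectors, rather than the pawn's.
; MouseY and MouseX feed straight into the controller's pitch and yaw input.
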(event Input|AxisEvents|InputAxisMoveForward
  (params (AxisValue :type Float%20%28single-precision%29))
  ;[1 1 1] 앞,뒤 이동
  (Pawn|Input|AddMovementInput (Game|Player|GetPlayerPawn 0) (Transformation|GetActorForwardVector) AxisValue false))

(event Input|AxisEvents|InputAxisMoveRight
  (params (AxisValue :type Float%20%28single-precision%29))
  ;[1 1 1] 양옆 이동
  (Pawn|Input|AddMovementInput (Game|Player|GetPlayerPawn 0) (Transformation|GetActorRightVector) AxisValue false))

(event Input|AxisEvents|InputAxisMouseX
  (params (AxisValue :type Float%20%28single-precision%29))
  ;[1 1 1] 양옆 회전
  (Class|PlayerController|AddYawInput AxisValue))

(event Input|AxisEvents|InputAxisMouseY
  (params (AxisValue :type Float%20%28single-precision%29))
  ;[1 1 1] 위아래 회전
  (Class|PlayerController|AddPitchInput AxisValue))

(fn ConstructionScript)