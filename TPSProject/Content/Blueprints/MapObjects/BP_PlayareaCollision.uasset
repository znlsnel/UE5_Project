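; BP_PlayareaCollision is a play-area boundary that warns the player with out-of-zone text on contact.
; It creates a WB_OutZoneText widget at BeginPlay, and a Box hit by a locally controlled BP_TPSPlayer calls its BeginWidget, then EndWidget three seconds later.
; An in-viewport check prevents repeat triggers.
; If the widget is invalid, that hit only recreates it without showing it.
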(event OnComponentHit(Box)
  (params (HitComponent :type Primitive%20Component%20Object%20Reference) (OtherActor :type Actor%20Object%20Reference) (OtherComp :type Primitive%20Component%20Object%20Reference) (NormalImpulse :type Vector :default "0, 0, 0") (Hit :type Hit%20Result%20Structure%20%28by%20ref%29))
  (bind _asbp_tpsplayer (Utilities|Casting|CastToBP_TPSPlayer OtherActor))
  (if (Pawn|IsLocallyControlled _asbp_tpsplayer)
    (Utilities|IsValid (Variables|Default|GetoutZoneTexet)
      (:Is%20Valid
        (if (not (UserInterface|Viewport|IsinViewport (Variables|Default|GetoutZoneTexet)))
          (Default|BeginWidget (Variables|Default|GetoutZoneTexet))
          (Utilities|FlowControl|Delay 3.0)
          (Default|EndWidget (Variables|Default|GetoutZoneTexet))))
      (:Is%20Not%20Valid
        (bind _returnvalue (UserInterface|CreateWidget "/Game/Assets/UI/WB_OutZoneText.WB_OutZoneText_C"))
        (Variables|Default|SetoutZoneTexet _returnvalue)))))

(event EventBeginPlay
  (bind _returnvalue (UserInterface|CreateWidget "/Game/Assets/UI/WB_OutZoneText.WB_OutZoneText_C"))
  (Variables|Default|SetoutZoneTexet _returnvalue))

(event Collision|EventActorBeginOverlap
  (params (OtherActor :type Actor%20Object%20Reference)))

(event EventTick
  (params (DeltaSeconds :type Float%20%28single-precision%29)))

(fn ConstructionScript)