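; BP_InteractableActor is an interactable actor that shows or hides an on-screen interaction marker.
; ToggleWidget lazily creates a WB_InteractableMark widget, caches it and adds it to the viewport when opened.
; Closing prints a debug "Hello" and removes the cached widget from the viewport.
; BeginPlay, overlap, Tick and the construction script are empty, and nothing in this Blueprint calls ToggleWidget.
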(event EventBeginPlay)

(event Collision|EventActorBeginOverlap
  (params (OtherActor :type Actor%20Object%20Reference)))

(event EventTick
  (params (DeltaSeconds :type Float%20%28single-precision%29)))

(event EventToggleWidget
  (params (open :type Boolean))
  (if open
    (Utilities|IsValid (Variables|Default|GetInteractableMark)
      (:Is%20Valid
        _)
      (:Is%20Not%20Valid
        (bind _returnvalue (UserInterface|CreateWidget "/Game/Assets/UI/WB_InteractableMark.WB_InteractableMark_C"))
        (Variables|Default|SetInteractableMark _returnvalue)))
    (if (not (UserInterface|Viewport|IsinViewport (Variables|Default|GetInteractableMark)))
      (UserInterface|Viewport|AddtoViewport (Variables|Default|GetInteractableMark) 0))
    (else
      (Development|PrintString "Hello")
      (Utilities|IsValid (Variables|Default|GetInteractableMark)
        (:Is%20Valid
          (if (UserInterface|Viewport|IsinViewport (Variables|Default|GetInteractableMark))
            (Widget|RemovefromParent (Variables|Default|GetInteractableMark))))))))

(fn ConstructionScript)