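; BP_StoneHead is an NPC that shows a dialog UI when interacted with.
; The Interaction event lazily creates a WB_Dialog widget, caches it, and opens it unless it is already in the viewport.
; When a BP_TPSPlayer leaves InteractionCollision, the NPC unbinds that player and closes any visible dialog if the player is locally controlled.
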(event OnComponentEndOverlap(InteractionCollision)
  (params (OverlappedComponent :type Primitive%20Component%20Object%20Reference) (OtherActor :type Actor%20Object%20Reference) (OtherComp :type Primitive%20Component%20Object%20Reference) (OtherBodyIndex :type Integer))
  (bind _asbp_tpsplayer (Utilities|Casting|CastToBP_TPSPlayer OtherActor))
  (Class|InteractableActor|UnBindPlayer _asbp_tpsplayer)
  (Utilities|IsValid (Variables|Default|GetDialogWidget)
    (:Is%20Valid
      (if (and (Pawn|IsLocallyControlled _asbp_tpsplayer) (UserInterface|Viewport|IsinViewport (Variables|Default|GetDialogWidget)))
        (Default|CloseWidget (Variables|Default|GetDialogWidget))))))

(event EventBeginPlay)

(event Collision|EventActorBeginOverlap
  (params (OtherActor :type Actor%20Object%20Reference)))

(event EventTick
  (params (DeltaSeconds :type Float%20%28single-precision%29)))

(event EventInteraction
  (if true
    (Utilities|IsValid (Variables|Default|GetDialogWidget)
      (:Is%20Valid
        (if (not (UserInterface|Viewport|IsinViewport (Variables|Default|GetDialogWidget)))
          (Default|OpenWIdget (Variables|Default|GetDialogWidget) :!label _label)))
      (:Is%20Not%20Valid
        (bind _returnvalue (UserInterface|CreateWidget "/Game/Assets/UI/NPC/Store/WB_Dialog.WB_Dialog_C"))
        (bind _output_get (Variables|Default|SetDialogWidget _returnvalue))
        (Utilities|IsValid _output_get
          (:Is%20Valid
            (goto _label)))))))

(fn ConstructionScript)