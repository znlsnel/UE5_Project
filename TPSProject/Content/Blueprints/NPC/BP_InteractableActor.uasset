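; Interactable actor in the NPC folder that shows and hides an on-screen interaction mark widget.
; InteractionCollision begin overlap passes a locally controlled BP_TPSPlayer to BindPlayer, which is defined outside this graph.
; ToggleWidget lazily creates and caches WB_InteractableMark, adds it to the viewport on open and removes it on close, where a debug "Hello" print remains.
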(event OnComponentBeginOverlap(InteractionCollision)
  (params (OverlappedComponent :type Primitive%20Component%20Object%20Reference) (OtherActor :type Actor%20Object%20Reference) (OtherComp :type Primitive%20Component%20Object%20Reference) (OtherBodyIndex :type Integer) (bFromSweep :type Boolean) (SweepResult :type Hit%20Result%20Structure%20%28by%20ref%29))
  (bind _asbp_tpsplayer (Utilities|Casting|CastToBP_TPSPlayer OtherActor))
  (Utilities|IsValid _asbp_tpsplayer
    (:Is%20Valid
      (if (Pawn|IsLocallyControlled _asbp_tpsplayer)
        (Class|InteractableActor|BindPlayer _asbp_tpsplayer)))))

(event EventBeginPlay)

(event Collision|EventActorBeginOverlap
  (params (OtherActor :type Actor%20Object%20Reference)))

(event EventTick
  (params (DeltaSeconds :type Float%20%28single-precision%29)))

(event EventToggleWidget
  (params (open :type Boolean))
  (if open
    (Utilities|IsValid (Variables|Default|GetInteractableMark)
      (:Is%20Valid
        _)
      (:Is%20Not%20Valid
        (bind _returnvalue (UserInterface|CreateWidget "/Game/Assets/UI/WB_InteractableMark.WB_InteractableMark_C"))
        (Variables|Default|SetInteractableMark _returnvalue)))
    (if (not (UserInterface|Viewport|IsinViewport (Variables|Default|GetInteractableMark)))
      (UserInterface|Viewport|AddtoViewport (Variables|Default|GetInteractableMark) 0))
    (else
      (Development|PrintString "Hello")
      (Utilities|IsValid (Variables|Default|GetInteractableMark)
        (:Is%20Valid
          (if (UserInterface|Viewport|IsinViewport (Variables|Default|GetInteractableMark))
            (Widget|RemovefromParent (Variables|Default|GetInteractableMark))))))))

(fn ConstructionScript)