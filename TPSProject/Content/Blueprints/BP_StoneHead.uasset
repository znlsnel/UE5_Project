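; BP_StoneHead is an interactable stone head actor that shows a dialog widget to the player.
; Its PlayerOverlap component binds a locally controlled BP_TPSPlayer on entering and unbinds any BP_TPSPlayer on leaving.
; The Interaction event lazily creates the Dialog widget, reuses it afterward, and opens it.
; Leaving the overlap also closes the open dialog for the local player.
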(event OnComponentBeginOverlap(PlayerOverlap)
  (params (OverlappedComponent :type Primitive%20Component%20Object%20Reference) (OtherActor :type Actor%20Object%20Reference) (OtherComp :type Primitive%20Component%20Object%20Reference) (OtherBodyIndex :type Integer) (bFromSweep :type Boolean) (SweepResult :type Hit%20Result%20Structure%20%28by%20ref%29))
  (bind _asbp_tpsplayer (Utilities|Casting|CastToBP_TPSPlayer OtherActor))
  (Utilities|IsValid _asbp_tpsplayer
    (:Is%20Valid
      (if (Pawn|IsLocallyControlled _asbp_tpsplayer)
        (Class|InteractableActor|BindPlayer _asbp_tpsplayer)))))

(event OnComponentEndOverlap(PlayerOverlap)
  (params (OverlappedComponent :type Primitive%20Component%20Object%20Reference) (OtherActor :type Actor%20Object%20Reference) (OtherComp :type Primitive%20Component%20Object%20Reference) (OtherBodyIndex :type Integer))
  (bind _asbp_tpsplayer (Utilities|Casting|CastToBP_TPSPlayer OtherActor))
  (Class|InteractableActor|UnBindPlayer _asbp_tpsplayer)
  (Utilities|IsValid (Variables|Default|GetDialogWidget)
    (:Is%20Valid
      (if (and (Pawn|IsLocallyControlled _asbp_tpsplayer) (UserInterface|Viewport|IsinViewport (Variables|Default|GetDialogWidget)))
        (Default|CloseWidget (Variables|Default|GetDialogWidget))))))

(event EventBeginPlay)

(event Collision|EventActorBeginOverlap
  (params (OtherActor :type Actor%20Object%20Reference)))

(event EventTick
  (params (DeltaSeconds :type Float%20%28single-precision%29)))

(event EventInteraction
  (if true
    (Utilities|IsValid (Variables|Default|GetDialogWidget)
      (:Is%20Valid
        (if (not (UserInterface|Viewport|IsinViewport (Variables|Default|GetDialogWidget)))
          (Default|OpenWIdget (Variables|Default|GetDialogWidget) :!label _label)))
      (:Is%20Not%20Valid
        (bind _returnvalue (UserInterface|CreateWidget "/Game/Assets/UI/Dialog.Dialog_C"))
        (bind _output_get (Variables|Default|SetDialogWidget _returnvalue))
        (Utilities|IsValid _output_get
          (:Is%20Valid
            (goto _label)))))))

(fn ConstructionScript)