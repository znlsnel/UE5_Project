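; Game state Blueprint that runs a day-night cycle by rotating the level's sun.
; BeginPlay finds a DirectionalLight and, if it is valid, starts a self-calling UpdateRotation event on a short Delay instead of Tick.
; Each step turns the light faster while its pitch is above about one degree, when it points upward, so night passes quicker.
; An unconnected BP_StoneWall spawn node never runs.
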(event Custom|UpdateRotation
  (bind _mysun (Variables|Default|GetMySun))
  (bind _rootcomponent (Variables|/Script/Engine.Actor|GetRootComponent _mysun))
  (if (> (.pitch (Transformation|GetWorldRotation _rootcomponent)) 1.0)
    (Transformation|AddWorldRotation _rootcomponent "0.300000, 0, 0" false false)
    (else
      (Transformation|AddWorldRotation _rootcomponent "0.100000, 0, 0" false false)))
  (Utilities|FlowControl|Delay 0.2)
  (CallFunction|UpdateRotation))

(event EventBeginPlay
  (bind _returnvalue (Actor|GetActorOfClass "/Script/Engine.DirectionalLight"))
  (bind _output_get (Variables|Default|SetMySun _returnvalue))
  (Utilities|IsValid _output_get
    (:Is%20Valid
      (CallFunction|UpdateRotation))))

(event EventTick
  (params (DeltaSeconds :type Float%20%28single-precision%29)))

(fn ConstructionScript)