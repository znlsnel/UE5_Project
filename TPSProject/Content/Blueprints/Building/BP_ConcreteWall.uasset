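; BP_ConcreteWall is a building Blueprint for a breakable concrete barrier with a shield value, built on a Geometry Collection.
; InitItem refills Shield to MaxShield and turns off the collection's physics and collision.
; DestroyActor sets IsDestroy, enables collision and physics simulation on the collection, then hides the actor after a short delay instead of removing it.
; No damage handling appears in this graph.
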(event Collision|EventActorBeginOverlap
  (params (OtherActor :type Actor%20Object%20Reference)))

(event EventTick
  (params (DeltaSeconds :type Float%20%28single-precision%29)))

(event EventDestroyActor
  (bind _s_old_concrete_barrier_vkurdfd_lod3_var1_geometrycollection (Variables|Default|GetS_Old_Concrete_Barrier_vkurdfd_lod3_Var1_GeometryCollection))
  (Variables|Default|SetisDestroy true)
  (Collision|SetCollisionEnabled _s_old_concrete_barrier_vkurdfd_lod3_var1_geometrycollection "QueryAndPhysics")
  (Physics|SetSimulatePhysics _s_old_concrete_barrier_vkurdfd_lod3_var1_geometrycollection true)
  (Utilities|FlowControl|Delay 3.0)
  (Rendering|SetActorHiddenInGame true))

(event EventInitItem
  (bind _s_old_concrete_barrier_vkurdfd_lod3_var1_geometrycollection (Variables|Default|GetS_Old_Concrete_Barrier_vkurdfd_lod3_Var1_GeometryCollection))
  (Physics|SetSimulatePhysics _s_old_concrete_barrier_vkurdfd_lod3_var1_geometrycollection false)
  (Variables|Default|Setshield (Variables|Default|GetMaxShield))
  (Collision|SetCollisionEnabled _s_old_concrete_barrier_vkurdfd_lod3_var1_geometrycollection "NoCollision"))

(fn ConstructionScript)