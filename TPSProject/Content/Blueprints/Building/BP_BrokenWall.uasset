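; Breakable wall building piece that collapses through a Geometry Collection when destroyed.
; InitItem sets Shield to MaxShield and keeps the collection non-simulating with collision off.
; DestroyActor forwards to DestroyActorServer, which shows only a same-named call and no direct link to DestroyActorMulti.
; DestroyActorMulti flags IsDestroy, enables collision and physics on the pieces, then hides the actor after a short delay.
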(event Custom|DestroyActorServer
  (CallFunction|DestroyActorServer))

(event Custom|DestroyActorMulti
  (bind _s_broken_wall_slund_lod3_geometrycollection (Variables|Default|GetS_Broken_Wall_slund_lod3_GeometryCollection))
  (Variables|Default|SetisDestroy true)
  (Collision|SetCollisionEnabled _s_broken_wall_slund_lod3_geometrycollection "QueryAndPhysics")
  (Physics|SetSimulatePhysics _s_broken_wall_slund_lod3_geometrycollection true)
  (Utilities|FlowControl|Delay 3.0)
  (Rendering|SetActorHiddenInGame true))

(event Collision|EventActorBeginOverlap
  (params (OtherActor :type Actor%20Object%20Reference)))

(event EventTick
  (params (DeltaSeconds :type Float%20%28single-precision%29)))

(event EventDestroyActor
  (CallFunction|DestroyActorServer))

(event EventInitItem
  (bind _s_broken_wall_slund_lod3_geometrycollection (Variables|Default|GetS_Broken_Wall_slund_lod3_GeometryCollection))
  (Physics|SetSimulatePhysics _s_broken_wall_slund_lod3_geometrycollection false)
  (Variables|Default|Setshield (Variables|Default|GetMaxShield))
  (Collision|SetCollisionEnabled _s_broken_wall_slund_lod3_geometrycollection "NoCollision"))

(fn ConstructionScript)