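; BP_StoneWall is a destructible stone wall building piece made of two Geometry Collection components.
; InitItem turns physics simulation off on both pieces to hold the wall in place.
; DestroyEvent turns physics simulation on for both so the wall collapses, then destroys the actor after a short delay.
; The IsDestroy flag and hide-in-game nodes are disconnected and never run.
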(event EventDestroyEvent
  (Utilities|FlowControl|Sequence
    (:then_0
      (Physics|SetSimulatePhysics (Variables|Default|GetS_Japanese_Stone_Wall_vfvndg3cb_lod3_Var1_GeometryCollection) true))
    (:then_1
      (Physics|SetSimulatePhysics (Variables|Default|GetS_Japanese_Stone_Wall_vfvndg3cb_lod3_Var1_GeometryCollection1) true)
      (Utilities|FlowControl|Delay 2.0)
      (Actor|DestroyActor))))

(event Collision|EventActorBeginOverlap
  (params (OtherActor :type Actor%20Object%20Reference)))

(event EventTick
  (params (DeltaSeconds :type Float%20%28single-precision%29)))

(event EventInitItem
  (Utilities|FlowControl|Sequence
    (:then_0
      (Physics|SetSimulatePhysics (Variables|Default|GetS_Japanese_Stone_Wall_vfvndg3cb_lod3_Var1_GeometryCollection) false))
    (:then_1
      (Physics|SetSimulatePhysics (Variables|Default|GetS_Japanese_Stone_Wall_vfvndg3cb_lod3_Var1_GeometryCollection1) false))))

(fn ConstructionScript)