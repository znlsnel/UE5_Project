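; Sandbag wall building piece with a shield value that collapses as a physics object when destroyed.
; InitItem refills the shield and turns off the barrier mesh's collision and physics.
; DestroyActor routes to DestroyActorServer, which only calls its own name; nothing here invokes DestroyActorMulti.
; DestroyActorMulti flags destruction, enables mesh collision and physics, then hides the actor after a delay without destroying it.
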(event Custom|DestroyActorServer
  (CallFunction|DestroyActorServer))

(event Custom|DestroyActorMulti
  (bind _s_sandbag_barrier_udtvegsfa_lod3_var1 (Variables|Default|GetS_Sandbag_Barrier_udtvegsfa_lod3_Var1))
  (Variables|Default|SetisDestroy true)
  (Collision|SetCollisionEnabled _s_sandbag_barrier_udtvegsfa_lod3_var1 "QueryAndPhysics")
  (Physics|SetSimulatePhysics _s_sandbag_barrier_udtvegsfa_lod3_var1 true)
  (Utilities|FlowControl|Delay 3.0)
  (Rendering|SetActorHiddenInGame true))

(event Collision|EventActorBeginOverlap
  (params (OtherActor :type Actor%20Object%20Reference)))

(event EventTick
  (params (DeltaSeconds :type Float%20%28single-precision%29)))

(event EventDestroyActor
  (CallFunction|DestroyActorServer))

(event EventInitItem
  (bind _s_sandbag_barrier_udtvegsfa_lod3_var1 (Variables|Default|GetS_Sandbag_Barrier_udtvegsfa_lod3_Var1))
  (Physics|SetSimulatePhysics _s_sandbag_barrier_udtvegsfa_lod3_var1 false)
  (Variables|Default|Setshield (Variables|Default|GetMaxShield))
  (Collision|SetCollisionEnabled _s_sandbag_barrier_udtvegsfa_lod3_var1 "NoCollision"))

(fn ConstructionScript)